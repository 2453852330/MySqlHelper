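; Example actor that sets up a MySQL connection and shows a UI for it on BeginPlay.
; It constructs a MySqlObject, points it at a local server with hardcoded root credentials and sets the library name.
; It then enables the mouse cursor and adds a UI_MYSQL widget to the viewport, passing that MySQL object in for the widget to use.
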(event `self.ReceiveBeginPlay`
  (bind _returnvalue (`GameplayStatics.GetPlayerController` 0))
  (`|ExecutionSequence`
    (:`then_0`
      (bind _returnvalue_2 (`|GenericCreateObject` "/Script/MySqlHelper.MySqlObject" self))
      (bind _output_get (set `self.MySql` _returnvalue_2))
      (`MySqlObject.UpdateSqlConnect` _output_get "localhost" 33060 "root" "123456")
      (`MySqlObject.SetLibName` _output_get "hello"))
    (:`then_1`
      (set `PlayerController.bShowMouseCursor` true _returnvalue)
      (bind _returnvalue_3 (`|CreateWidget` "/MySqlHelper/UI_MySql.UI_MYSQL_C" _returnvalue (`self.MySql`)))
      (`UserWidget.AddToViewport` _returnvalue_3 0))))

(fn `UserConstructionScript`)